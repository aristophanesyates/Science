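; BP_Scientist is a player-controlled pawn with world-axis movement driven by the UpDown and LeftRight inputs.
; Each axis event feeds movement input along world X or Y, independent of where the pawn faces.
; While input is non-zero, Tick turns the Cone component toward the input direction using a shortest-path rotator lerp scaled by RotationSpeed and delta time.
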(event EventBeginPlay)

(event Collision|EventActorBeginOverlap
  (params (OtherActor :type Actor%20Object%20Reference)))

(event EventTick
  (params (DeltaSeconds :type Float%20%28single-precision%29))
  (if (or (!= (Input|AxisValues|GetLeftRight) 0.0) (!= (Input|AxisValues|GetUpDown) 0.0))
    (Variables|Default|SetDirection (Math|Vector|MakeVector (Input|AxisValues|GetUpDown) (Input|AxisValues|GetLeftRight) 0.0))
    (Transformation|SetWorldRotation (Variables|Default|GetCone) (Math|Rotator|Lerp(Rotator) (Transformation|GetWorldRotation (Variables|Default|GetCone)) (Math|Conversions|RotationFromXVector (Variables|Default|GetDirection)) (* (Variables|Default|GetrotationSpeed) DeltaSeconds) true) false false)))

(event Input|AxisEvents|InputAxisUpDown
  (params (AxisValue :type Float%20%28single-precision%29))
  (Pawn|Input|AddMovementInput "1.000000, 0, 0" AxisValue false))

(event Input|AxisEvents|InputAxisLeftRight
  (params (AxisValue :type Float%20%28single-precision%29))
  (Pawn|Input|AddMovementInput "0,1.000000, 0" AxisValue false))

(fn ConstructionScript)